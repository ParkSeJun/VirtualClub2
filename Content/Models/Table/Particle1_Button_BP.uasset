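; Table button actor that toggles a set of particle effects and its own highlight color when OnTriggerPressed fires.
; After a short delay, pressing recolors the Cube through a dynamic material and spawns four sprite emitters at hardcoded locations; pressing again clears the color and destroys them.
; A long delay also resets the pressed flag, leaving emitters active.
; MoveComponentTo offsets are zero, and overlap-triggered character paths are disconnected.
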(event OnComponentBeginOverlap(Box)
  (params (OverlappedComponent :type Primitive%20Component%20Object%20Reference) (OtherActor :type Actor%20Object%20Reference) (OtherComp :type Primitive%20Component%20Object%20Reference) (OtherBodyIndex :type Integer) (bFromSweep :type Boolean) (SweepResult :type Hit%20Result%20Structure%20%28by%20ref%29)))

(event EventBeginPlay)

(event Collision|EventActorBeginOverlap
  (params (OtherActor :type Actor%20Object%20Reference)))

(event EventTick
  (params (DeltaSeconds :type Float%20%28single-precision%29)))

(event EventOnTriggerPressed
  (params (Controller :type Motion%20Controller%20Component%20Object%20Reference))
  (bind _cube (Variables|Default|GetCube))
  (bind _cube_2 (Variables|Default|GetCube))
  (bind _returnvalue (Transformation|GetRelativeTransform _cube_2))
  (bind _returnvalue_2 (Transformation|GetRelativeTransform _cube))
  (Utilities|FlowControl|Delay 0.2)
  (if (Variables|Default|Getis_pressed)
    (bind _returnvalue_3 (Rendering|Material|CreateDynamicMaterialInstance (Variables|Default|GetCube) 0 0 "None" :!class /Script/Engine.PrimitiveComponent))
    (Rendering|Material|SetVectorParameterValue _returnvalue_3 "ButtonParam" (Utilities|Struct|MakeLinearColor 0.0 0.0 0.0 0.0) :!class /Script/Engine.MaterialInstanceDynamic)
    (Components|DestroyComponent (stale _returnvalue_8))
    (else
      (bind _returnvalue_4 (Rendering|Material|CreateDynamicMaterialInstance (Variables|Default|GetCube) 0 0 "None" :!class /Script/Engine.PrimitiveComponent))
      (Rendering|Material|SetVectorParameterValue _returnvalue_4 "ButtonParam" (Utilities|Struct|MakeLinearColor 5.0 0.0 0.0 0.0) :!class /Script/Engine.MaterialInstanceDynamic)
      (Variables|Default|Setis_pressed true)
      (Components|MoveComponentTo _cube (- (.location _returnvalue_2) "0, 0, 0") (.rotation _returnvalue_2) false false 0.5 false)
      (bind _returnvalue_5 (Effects|SpawnEmitteratLocation "/Game/Particle/P_Sprite.P_Sprite" "-790.000000,-660.000000,-209.000000"))
      (bind _returnvalue_6 (Effects|SpawnEmitteratLocation "/Game/Particle/P_Sprite.P_Sprite" "-784.000000,-1580.000000,-13.000000"))
      (bind _returnvalue_7 (Effects|SpawnEmitteratLocation "/Game/Particle/P_Sprite.P_Sprite" "711.000000,-1571.000000,-13.000000"))
      (bind _returnvalue_8 (Effects|SpawnEmitteratLocation "/Game/Particle/P_Sprite.P_Sprite" "691.000000,-656.000000,-209.000000"))
      (Utilities|FlowControl|Delay 2e+02)))
  (Components|MoveComponentTo _cube_2 (+ (.location _returnvalue) "0, 0, 0") (.rotation _returnvalue) false false 1.0 false)
  (Variables|Default|Setis_pressed false))

(fn ConstructionScript)