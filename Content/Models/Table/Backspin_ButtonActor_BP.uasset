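; Backspin button actor on a table with left and right records, toggling reverse playback for its side when the VR controller trigger is pressed.
; The press calls the parent handler, then IsLeftRecord selects which reverse state to flip through NewGameMode.
; Construction creates a dynamic material instance for the Outliner.
; Unconnected leftover logic holds drag-based play-time scrubbing, pitch reset and outline visibility on touch.
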(event EventBeginPlay)

(event Collision|EventActorBeginOverlap
  (params (OtherActor :type Actor%20Object%20Reference)))

(event EventTick
  (params (DeltaSeconds :type Float%20%28single-precision%29)))

(event EventOnTriggerPressed
  (params (Controller :type Motion%20Controller%20Component%20Object%20Reference))
  (bind _returnvalue (Game|GetGameMode))
  (bind _asnew_game_mode (Utilities|Casting|CastToNewGameMode _returnvalue))
  (|CallParentFunction Controller)
  (if (Variables|Default|GetisLeftRecord)
    (Default|OnPlayReverse1 _asnew_game_mode (not (Variables|/Game/NewGameMode.NewGameMode_C|GetisReverse1 _asnew_game_mode)))
    (else
      (Default|OnPlayReverse2 _asnew_game_mode (not (Variables|/Game/NewGameMode.NewGameMode_C|GetisReverse2 _asnew_game_mode))))))

(event EventOnTriggerReleased)

(fn ConstructionScript
  (bind _outliner (Variables|Default|Getoutliner))
  (bind _returnvalue (Rendering|Material|CreateDynamicMaterialInstance _outliner 0 (Rendering|Material|GetMaterial _outliner 0) "None" :!class /Script/Engine.PrimitiveComponent))
  (Variables|Default|SetoutlinerMID _returnvalue))