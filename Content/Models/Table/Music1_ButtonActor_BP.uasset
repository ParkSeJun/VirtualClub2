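; Music button actor that toggles on box overlap, spawning a SoundMater_BP at a fixed location to play music.
; After a short delay, a press tints the Cube red via a dynamic material; only Character_A triggers the spawn, though any actor flips the state.
; Pressing again clears the tint and stops the audio, while a long timeout after spawning only resets the pressed state.
; MoveComponentTo calls use zero offsets, so the Cube stays in place.
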(event OnComponentBeginOverlap(Box)
  (params (OverlappedComponent :type Primitive%20Component%20Object%20Reference) (OtherActor :type Actor%20Object%20Reference) (OtherComp :type Primitive%20Component%20Object%20Reference) (OtherBodyIndex :type Integer) (bFromSweep :type Boolean) (SweepResult :type Hit%20Result%20Structure%20%28by%20ref%29))
  (bind _cube (Variables|Default|GetCube))
  (bind _cube_2 (Variables|Default|GetCube))
  (bind _returnvalue (Transformation|GetRelativeTransform _cube_2))
  (bind _returnvalue_2 (Transformation|GetRelativeTransform _cube))
  (Utilities|FlowControl|Delay 0.2)
  (if (Variables|Default|Getis_pressed)
    (bind _returnvalue_3 (Rendering|Material|CreateDynamicMaterialInstance (Variables|Default|GetCube) 0 0 "None" :!class /Script/Engine.PrimitiveComponent))
    (Rendering|Material|SetVectorParameterValue _returnvalue_3 "ButtonParam" (Utilities|Struct|MakeLinearColor 0.0 0.0 0.0 0.0) :!class /Script/Engine.MaterialInstanceDynamic)
    (Audio|Components|Audio|Stop (Variables|/Game/Sound/SoundMater_BP.SoundMater_BP_C|GetAudio (stale _returnvalue_5)))
    (else
      (bind _returnvalue_4 (Rendering|Material|CreateDynamicMaterialInstance (Variables|Default|GetCube) 0 0 "None" :!class /Script/Engine.PrimitiveComponent))
      (Rendering|Material|SetVectorParameterValue _returnvalue_4 "ButtonParam" (Utilities|Struct|MakeLinearColor 5.0 0.0 0.0 0.0) :!class /Script/Engine.MaterialInstanceDynamic)
      (Variables|Default|Setis_pressed true)
      (Utilities|Casting|CastToCharacter_A OtherActor)
      (Components|MoveComponentTo _cube (- (.location _returnvalue_2) "0, 0, 0") (.rotation _returnvalue_2) false false 0.5 false)
      (bind _returnvalue_5 (Game|SpawnActorfromClass "/Game/Sound/SoundMater_BP.SoundMater_BP_C" (Math|Transform|MakeTransform "-894.000000,-1591.822266,567.844238" "0, 0, 0" "1,1,1") "Undefined" 0 0))
      (Utilities|FlowControl|Delay 2e+02)))
  (Components|MoveComponentTo _cube_2 (+ (.location _returnvalue) "0, 0, 0") (.rotation _returnvalue) false false 1.0 false)
  (Variables|Default|Setis_pressed false))

(event EventBeginPlay)

(event Collision|EventActorBeginOverlap
  (params (OtherActor :type Actor%20Object%20Reference)))

(event EventTick
  (params (DeltaSeconds :type Float%20%28single-precision%29)))

(fn ConstructionScript)