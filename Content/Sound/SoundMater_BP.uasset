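; SoundMater_BP is an audio visualizer actor that plays a sound and spawns AudioElement_BP actors scaled by its spectrum.
; Playback percent updates become elapsed time, which samples normalized Constant-Q data for channel 0 from ConstantRef.
; Band values set the Z scale of actors spawned at the root location.
; A Delay sits inside the band loop, so calls made while it is pending do not spawn separately.
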(event Custom|PlaybackChange
  (params (PlayingSoundWave :type Sound%20Wave%20Object%20Reference) (PlaybackPercent :type Float%20%28single-precision%29))
  (Variables|Default|SetPlayedTime (* PlaybackPercent (Variables|Default|GetDuration_0)))
  (for _array_element (Class|ConstantQNRT|GetNormalizedChannelConstantQatTime (Variables|Default|GetConstant_Ref) (Variables|Default|GetPlayedTime))
    (Utilities|FlowControl|Delay 0.05)
    (Game|SpawnActorfromClass "/Game/Sound/AudioElement_BP.AudioElement_BP_C" (Math|Transform|MakeTransform (Transformation|GetWorldLocation (Variables|Default|GetDefaultSceneRoot)) "0, 0, 0" (Math|Vector|MakeVector 0.2 0.2 (* _array_element 1e+01))) "Undefined" 0 0)))

(event EventBeginPlay
  (Audio|Components|Audio|SetSound (Variables|Default|GetAudio) (Variables|Default|GetNew%20Sound))
  (Variables|Default|SetDuration_0 (Variables|/Script/Engine.SoundBase|GetDuration (Variables|Default|GetNew%20Sound)))
  (EventDispatchers|BindEventtoOnAudioPlaybackPercent (Variables|Default|GetAudio) (delegate Custom|PlaybackChange))
  (Audio|Components|Audio|Play (Variables|Default|GetAudio) 0.0))

(fn ConstructionScript)