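; BP_Sound is an audio visualizer actor that drives a row of cubes as a spectrum display for a music track.
; On BeginPlay it assigns the track, spawns cubes along Y and collects all BP_cube actors; P starts playback or toggles pause.
; Each playback-percent callback converts progress to seconds, samples precomputed Audio Synesthesia Constant-Q data and sets each cube's Z scale from its band strength.
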(event Custom|onPlaybackChange
  (params (PlayingSoundWave :type Sound%20Wave%20Object%20Reference) (PlaybackPercent :type Float%20%28single-precision%29))
  (CallFunction|SynesthesiaScaleCube (Variables|Default|GetMusicDuration) PlaybackPercent (Variables|Default|GetSound%20Cubes)))

(event EventBeginPlay
  (bind _returnvalue (Game|GetPlayerController 0))
  (bind _music (Variables|Default|GetMusic))
  (Utilities|FlowControl|Sequence
    (:then_0
      (Input|EnableInput _returnvalue)
      (Input|SetInputModeGameOnly _returnvalue))
    (:then_1
      (Variables|/Script/Engine.AudioComponent|SetSound (Variables|Default|GetAudio) _music)
      (Variables|Default|SetMusicDuration (Variables|/Script/Engine.SoundBase|GetDuration _music)))
    (:then_2
      (bind _soundcubes (CallFunction|SpawnSoundCube (Variables|Default|GetNumof%20Cube) (Variables|Default|GetCube%20Spacing)))
      (Variables|Default|SetSound%20Cubes _soundcubes))
    (:then_3
      (EventDispatchers|BindEventtoOnAudioPlaybackPercent (Variables|Default|GetAudio) (delegate Custom|onPlaybackChange)))))

(event Collision|EventActorBeginOverlap
  (params (OtherActor :type Actor%20Object%20Reference)))

(event EventTick
  (params (DeltaSeconds :type Float%20%28single-precision%29)))

(event Input|KeyboardEvents|P
  (params (Key :type Key%20Structure :default "None"))
  (bind _audio (Variables|Default|GetAudio))
  (:Pressed
    (if (Audio|Components|Audio|IsPlaying (Variables|Default|GetAudio))
      (bind _isa (Utilities|FlowControl|FlipFlop)
        (:A
          _)
        (:B
          _))
      (Class|AudioComponent|SetPaused _audio _isa)
      (else
        (Audio|Components|Audio|Play _audio 0.0)))))

(fn ConstructionScript)

(fn SpawnSoundCube
  (params (NumofCube :type Integer) (CubeSpacing :type Float%20%28single-precision%29))
  (bind _defaultsceneroot (Variables|Default|GetDefaultSceneRoot))
  (bind _returnvalue (Transformation|GetWorldLocation _defaultsceneroot))
  (for _index (range 1 NumofCube)
    (Game|SpawnActorfromClass "/Game/Sound/AudioVisualizer/BP_cube.BP_cube_C" (Math|Transform|MakeTransform (Math|Vector|MakeVector (.x _returnvalue) (+ (.y _returnvalue) (* _index CubeSpacing)) (.z _returnvalue)) "0, 0, 0" "0.100000,0.100000,0.100000") "Undefined" 0 0))
  (bind _outactors (Actor|GetAllActorsOfClass "/Game/Sound/AudioVisualizer/BP_cube.BP_cube_C"))
  (return _outactors))

(fn SynesthesiaScaleCube
  (params (MusicDuration :type Float%20%28single-precision%29) (PercentagePlayed :type Float%20%28single-precision%29) (SoundCubes :type Array%20of%20BP%20Cube%20Object%20References))
  (Utilities|FlowControl|Sequence
    (:then_0
      (Variables|Default|SetPosition%20Audio (* MusicDuration PercentagePlayed)))
    (:then_1
      (LocalVariables|SetFrequencyBandStrengths (Class|ConstantQNRT|GetNormalizedChannelConstantQatTime (Variables|Default|GetSynesthesiaAnalysis) (Variables|Default|GetPosition%20Audio))))
    (:then_2
      (for (_array_element _array_index) (LocalVariables|GetFrequencyBandStrengths)
        (Transformation|SetWorldScale3D (Variables|/Game/Sound/AudioVisualizer/BP_cube.BP_cube_C|GetCube (Utilities|Array|Get(acopy) SoundCubes _array_index)) (Math|Vector|MakeVector 0.1 0.1 (* _array_element (Variables|Default|GetScaling%20Factor))))))))