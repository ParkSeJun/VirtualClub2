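; Networked sound button that a player triggers by walking into its box, pressing it and playing a 2D sound.
; On non-authority machines, the overlap makes the locally controlled Character_A call CallOnSoundRPC with this button.
; The bound OnButtonPlay event animates the button down, plays the sound, waits a configurable delay, then raises it.
; An IsPressed flag blocks retriggering until the cycle ends.
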(event OnComponentBeginOverlap(Box)
  (params (OverlappedComponent :type Primitive%20Component%20Object%20Reference) (OtherActor :type Actor%20Object%20Reference) (OtherComp :type Primitive%20Component%20Object%20Reference) (OtherBodyIndex :type Integer) (bFromSweep :type Boolean) (SweepResult :type Hit%20Result%20Structure%20%28by%20ref%29))
  (Networking|SwitchHasAuthority
    (:Remote
      (bind _ascharacter_a (Utilities|Casting|CastToCharacter_A OtherActor))
      (if (Pawn|IsLocallyControlled _ascharacter_a)
        (Default|CallOnSoundRPC _ascharacter_a self)))))

(event Custom|OnButtonPlay_Event
  (bind _pressedlocation (Variables|Default|GetPressedLocation))
  (bind _releasedlocation (Variables|Default|GetReleasedLocation))
  (bind _returnvalue (Transformation|GetRelativeTransform _pressedlocation))
  (bind _returnvalue_2 (Transformation|GetRelativeTransform _releasedlocation))
  (if (not (Variables|Default|Getis_pressed))
    (Variables|Default|Setis_pressed true)
    (Components|MoveComponentTo (Variables|Default|Getbutton) (.location _returnvalue) (.rotation _returnvalue) false false 0.25 false)
    (Audio|PlaySound2D (Variables|Default|GetSoundBase) 1.0 1.0 0.0 0 0)
    (Utilities|FlowControl|Delay (Variables|Default|GetMyDelay))
    (Components|MoveComponentTo (Variables|Default|Getbutton) (.location _returnvalue_2) (.rotation _returnvalue_2) false false 0.5 false)
    (Variables|Default|Setis_pressed false)))

(event EventBeginPlay
  (EventDispatchers|BindEventtoOnButtonPlay (delegate Custom|OnButtonPlay_Event)))

(fn ConstructionScript)