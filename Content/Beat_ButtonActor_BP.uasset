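; Toggle button actor that switches a beat layer, either clap or kick/snare, on the player characters.
; Each trigger press flips IsPressed and recolors the cube through a new dynamic material instance's ButtonParam.
; It then sets IsBeatClap or IsBeatKickSnare, chosen by IsClap, on every Character_New tagged Player.
; Tick shows the outliner mesh only while IsTouching is true.
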(event EventBeginPlay)

(event Collision|EventActorBeginOverlap
  (params (OtherActor :type Actor%20Object%20Reference))
  (|CallParentFunction OtherActor))

(event EventTick
  (params (DeltaSeconds :type Float%20%28single-precision%29))
  (Development|SetHiddeninGame (Variables|Default|GetOutliner) (not (Variables|Default|GetisTouching)) false))

(event EventOnTriggerPressed
  (params (Controller :type Motion%20Controller%20Component%20Object%20Reference))
  (|CallParentFunction Controller)
  (if (Variables|Default|Getis_pressed)
    (bind _returnvalue (Rendering|Material|CreateDynamicMaterialInstance (Variables|Default|GetCube) 0 0 "None" :!class /Script/Engine.PrimitiveComponent))
    (Rendering|Material|SetVectorParameterValue _returnvalue "ButtonParam" (Utilities|Struct|MakeLinearColor 0.0 0.0 0.0 0.0) :!class /Script/Engine.MaterialInstanceDynamic)
    (Variables|Default|Setis_pressed false)
    (bind _outactors (Actor|GetAllActorswithTag "Player"))
    (for _array_element _outactors
      (if (Variables|Default|GetisClap)
        (Variables|/Game/FirstPersonCPP/Blueprints/Character_New.Character_New_C|SetIsBeatClap (.AsCharacter%20New (Utilities|Casting|CastToCharacter_New _array_element)) false)
        (else
          (Variables|/Game/FirstPersonCPP/Blueprints/Character_New.Character_New_C|SetIsBeatKickSnare (.AsCharacter%20New (Utilities|Casting|CastToCharacter_New _array_element)) false))))
    (else
      (bind _returnvalue_2 (Rendering|Material|CreateDynamicMaterialInstance (Variables|Default|GetCube) 0 0 "None" :!class /Script/Engine.PrimitiveComponent))
      (Rendering|Material|SetVectorParameterValue _returnvalue_2 "ButtonParam" (Utilities|Struct|MakeLinearColor 5.0 0.0 0.0 0.0) :!class /Script/Engine.MaterialInstanceDynamic)
      (Variables|Default|Setis_pressed true)
      (bind _outactors_2 (Actor|GetAllActorswithTag "Player"))
      (for _array_element_2 _outactors_2
        (if (Variables|Default|GetisClap)
          (Variables|/Game/FirstPersonCPP/Blueprints/Character_New.Character_New_C|SetIsBeatClap (.AsCharacter%20New (Utilities|Casting|CastToCharacter_New _array_element_2)) true)
          (else
            (Variables|/Game/FirstPersonCPP/Blueprints/Character_New.Character_New_C|SetIsBeatKickSnare (.AsCharacter%20New (Utilities|Casting|CastToCharacter_New _array_element_2)) true)))))))

(fn ConstructionScript
  (|CallParentFunction))