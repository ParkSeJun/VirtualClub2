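; ControllableButtonBP is a button actor that tracks motion-controller touch and trigger input.
; A trigger press claims the first controller as CurrentController and sets IsPressing; release clears both, while touch events toggle IsTouching.
; GetDifference returns the held controller's change in distance from StartPosition relative to StartDistance, or zero without one.
; The nodes that capture those start values are disconnected, and press and release print debug strings.
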(event Custom|OnTriggerPressed
  (params (Controller :type Motion%20Controller%20Component%20Object%20Reference))
  (Development|PrintString "pressed")
  (if (not (Utilities|IsValidSoftObjectReference (Variables|Default|GetcurrentController)))
    (bind _output_get (Variables|Default|SetcurrentController (Utilities|ResolveSoftReference Controller)))
    (Variables|Default|SetisPressing true)))

(event Custom|OnTouchEnter
  (Variables|Default|SetisTouching true))

(event Custom|OnTriggerReleased
  (Development|PrintString "release")
  (Variables|Default|SetcurrentController 0)
  (Variables|Default|SetisPressing false))

(event Custom|OnTouchEnd
  (Variables|Default|SetisTouching false))

(event Collision|EventActorBeginOverlap
  (params (OtherActor :type Actor%20Object%20Reference)))

(fn ConstructionScript)

(fn GetDifference
  (if (Utilities|IsValidSoftObjectReference (Variables|Default|GetcurrentController))
    (return (- (Math|Vector|Distance(Vector) (Variables|Default|GetstartPosition) (Transformation|GetWorldLocation (Utilities|ResolveSoftReference (Variables|Default|GetcurrentController)))) (Variables|Default|GetstartDistance)))
    (else
      (return 0.0))))