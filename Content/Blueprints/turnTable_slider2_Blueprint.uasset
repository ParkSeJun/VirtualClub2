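; A turntable slider actor that the player drags along the world Y axis with a controller.
; On trigger press it calls the parent handler and records the controller and slider Y positions.
; While pressed, Tick offsets the slider by the controller's movement, clamped to a range, and shows the outliner only while touched or pressed.
; Unconnected leftover nodes would swap the player character to the Jane mesh and animation Blueprint.
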(event EventBeginPlay)

(event Collision|EventActorBeginOverlap
  (params (OtherActor :type Actor%20Object%20Reference)))

(event EventTick
  (params (DeltaSeconds :type Float%20%28single-precision%29))
  (bind _returnvalue (Transformation|GetActorLocation))
  (bind _range (Variables|Default|GetRange))
  (Development|SetHiddeninGame (Variables|Default|Getoutliner) (not (or (Variables|Default|GetisTouching) (Variables|Default|GetisPressing))) false)
  (if (Variables|Default|GetisPressing)
    (Transformation|SetActorLocation (Math|Vector|MakeVector (.x _returnvalue) (Math|Float|Clamp(Float) (+ (- (.y (Transformation|GetWorldLocation (Utilities|ResolveSoftReference (Variables|Default|GetcurrentController)))) (Variables|Default|GetstartControllerY)) (Variables|Default|GetstartSliderY)) (.value (.lowerbound _range)) (.value (.upperbound _range))) (.z _returnvalue)) false false)))

(event EventOnTriggerPressed
  (params (Controller :type Motion%20Controller%20Component%20Object%20Reference))
  (|CallParentFunction Controller)
  (Variables|Default|SetstartControllerY (.y (Transformation|GetWorldLocation (Utilities|ResolveSoftReference (Variables|Default|GetcurrentController)))))
  (Variables|Default|SetstartSliderY (.y (Transformation|GetActorLocation))))

(fn ConstructionScript
  (|CallParentFunction))